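; Enemy character that spots the player by pawn sensing, fires spell projectiles from its head socket and closes in.
; Sighting a living player starts randomly delayed shots and an AI move, which loops back to shooting on arrival.
; Damage plays a hit sound and drains health shown on a widget bar.
; Death triggers ragdoll, a delayed particle effect and destruction, and heals the player, capped at full health.
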(event OnSeePawn(PawnSensing)
  (params (Pawn :type Pawn%20Object%20Reference))
  ;[1 1 1] Shoot projectile at the player, and move to the player
  (bind _asthird_person_character (Utilities|Casting|CastToThirdPersonCharacter Pawn))
  (bind _output_get (Variables|Default|SetPlayer _asthird_person_character))
  (if (and (not (Variables|Default|GetisDeadEnemy)) (> (Variables|/Game/Character/Blueprints/ThirdPersonCharacter.ThirdPersonCharacter_C|GetHealth _output_get) 0.0))
    (if (not (Variables|/Game/Character/Blueprints/ThirdPersonCharacter.ThirdPersonCharacter_C|GetisDead (Variables|Default|GetPlayer)))
      (Utilities|FlowControl|Delay (Math|Random|RandomFloatinRange 3.0 7.0) :!label _label)
      (Game|SpawnActorfromClass "/Game/Character/Blueprints/BP_Spell02.BP_Spell02_C" (Math|Transform|MakeTransform (Transformation|GetSocketLocation (Variables|Character|GetMesh) "headSocket") (Math|Rotator|FindLookatRotation (Transformation|GetActorLocation) (Transformation|GetActorLocation _asthird_person_character)) "1,1,1") "Undefined" 0 0)
      (Utilities|FlowControl|Delay (Math|Random|RandomFloatinRange 1.0 5.0))
      (Utilities|FlowControl|Sequence
        (:then_0
          (AI|AIMoveTo self "0, 0, 0" Pawn 2e+02 false
            (:OnSuccess
              (goto _label))))
        (:then_1
          (Transformation|SetActorRotation (Math|Rotator|FindLookatRotation (Transformation|GetActorLocation) (Transformation|GetActorLocation _asthird_person_character))))))))

(event Game|Damage|EventAnyDamage
  (params (Damage :type Float%20%28single-precision%29) (DamageType :type Damage%20Type%20Object%20Reference) (InstigatedBy :type Controller%20Object%20Reference) (DamageCauser :type Actor%20Object%20Reference))
  (bind _capsulecomponent (Variables|Collision|GetCapsuleComponent))
  (bind _player (Variables|Default|GetPlayer))
  ;[1 1 1] Receive damage from the player
  (Utilities|FlowControl|Sequence
    (:then_0
      ;;[1 1 1] emitt sound when hit
      (Audio|PlaySoundatLocation "/Game/Sounds/163447__under7dude__zombie-hit.163447__under7dude__zombie-hit" (Transformation|GetActorLocation) "0, 0, 0" 3.0 1.0 0.0 0 0 0))
    (:then_1
      (bind _output_get (Variables|Default|SetHealthEnemy (- (Variables|Default|GetHealthEnemy) Damage)))
      (if (<= _output_get 0.0)
        (Utilities|FlowControl|Sequence
          (:then_0
            (Variables|Default|SetisDeadEnemy true)
            (Physics|SetSimulatePhysics (Variables|Character|GetMesh) true)
            (Collision|SetCollisionProfileName (Variables|Character|GetMesh) "Ragdoll" :!class /Script/Engine.PrimitiveComponent)
            (Collision|SetCollisionResponsetoChannel (Variables|Character|GetMesh) "ECC_Pawn" "ECR_Block")
            (Rendering|SetVisibility (Variables|Default|GetWidget) false false)
            (Utilities|FlowControl|Delay 0.5)
            (Utilities|IsValid _capsulecomponent
              (:Is%20Valid
                (Components|DestroyComponent _capsulecomponent)
                (Utilities|FlowControl|Delay 2.0)
                (Utilities|FlowControl|Sequence
                  (:then_0
                    (Components|Activation|SetActive (Variables|Default|GetParticleSystem) true false))
                  (:then_1
                    (Utilities|FlowControl|Delay 0.6)
                    (Actor|DestroyActor))))))
          (:then_1
            ;;[1 1 1] Player receive 10 health points when kill an enemy
            (if (<= (+ (Variables|/Game/Character/Blueprints/ThirdPersonCharacter.ThirdPersonCharacter_C|GetHealth _player) 1e+01) 1e+02)
              (Variables|/Game/Character/Blueprints/ThirdPersonCharacter.ThirdPersonCharacter_C|SetHealth _player (+ (Variables|/Game/Character/Blueprints/ThirdPersonCharacter.ThirdPersonCharacter_C|GetHealth _player) 1e+01))
              (else
                (Variables|/Game/Character/Blueprints/ThirdPersonCharacter.ThirdPersonCharacter_C|SetHealth _player 1e+02)))))))))

(event EventTick
  (params (DeltaSeconds :type Float%20%28single-precision%29))
  ;[1 1 1] Enemy HUD
  (bind _ashud_enemy (Utilities|Casting|CastToHUD_Enemy (UserInterface|GetUserWidgetObject (Variables|Default|GetWidget))))
  (Progress|SetPercent (Variables|/Game/Character/Widgets/HUD_Enemy.HUD_Enemy_C|GetProgressBar_Enemy _ashud_enemy) (/ (Variables|Default|GetHealthEnemy) 1e+02)))

(fn ConstructionScript)